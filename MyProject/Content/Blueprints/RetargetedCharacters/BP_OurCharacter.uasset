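; BP_OurCharacter is a retargeted character Blueprint that plays a pickaxe attack animation on its Manny mesh.
; One tick after BeginPlay, it makes the root's first child component tick after the root's grandparent attach component, ordering updates when attached to another actor.
; PlayPickaxeAttack plays the attack montage without stopping other montages, using a flag to block re-triggering until it completes or is interrupted.
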(event `self.ReceiveBeginPlay`
  (bind _rootcomponent (`self.RootComponent`))
  (bind _returnvalue (`SceneComponent.GetAttachParent` _rootcomponent))
  (bind _returnvalue_2 (`SceneComponent.GetAttachParent` _returnvalue))
  (`|ExecutionSequence`
    (:`then_0`
      (`KismetSystemLibrary.DelayUntilNextTick`)
      (`/Engine/EditorBlueprintResources/StandardMacros.IsValid` _returnvalue
        (:`Is Valid`
          (`/Engine/EditorBlueprintResources/StandardMacros.IsValid` _returnvalue_2
            (:`Is Valid`
              (`ActorComponent.AddTickPrerequisiteComponent` (`SceneComponent.GetChildComponent` _rootcomponent 0) _returnvalue_2))))))))

(event `PlayPickaxeAttack`
  (if (not (`self.bPickaxeAttackPlaying`))
    (set `self.bPickaxeAttackPlaying` true)
    (`|PlayMontage` (`self.Manny`) "/Game/MainPlayer/Animations/AM_Pickaxe_Attack_Montage.AM_Pickaxe_Attack_Montage" 1.0 0.0 "None" false
      (:`OnCompleted`
        _)
      (:`OnInterrupted`
        _))
    (set `self.bPickaxeAttackPlaying` false)))

(fn `UserConstructionScript`)